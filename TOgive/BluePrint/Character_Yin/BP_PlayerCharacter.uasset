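; Player character Blueprint that relays health and mana changes to the UI.
; Health changes set the fill ratio on the character's own HealthBar widget, then on the health bar in the BP_PlayerControllerBase PrimaryUI.
; Mana changes update only the PrimaryUI mana bar.
; BeginPlay, overlap and Tick are disabled stubs, so the graph is purely event-driven.
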(event `self.BP_OnHealthChanged`
  (params (Health :type "Float (single-precision)") (MaxHealth :type "Float (single-precision)"))
  ;[1 1 1] UI
  ;[1 1 1] 血条显示
  (bind _ashealth_bar (cast `/Game/UI/HealthBar` (`WidgetComponent.GetUserWidgetObject` (`self.HealthBar`))))
  (`/Game/UI/HealthBar.SetPercentage` _ashealth_bar (/ Health MaxHealth))
  (bind _asbp_player_controller_base (cast `/Game/BluePrint/BP_PlayerControllerBase` (`self.GetController`)))
  (`/Game/UI/WBP_HealthBar.SetPercentage` (`/Game/UI/WBP_PrimaryUI.WBP_HealthBar` (`/Game/BluePrint/BP_PlayerControllerBase.Primary UI` _asbp_player_controller_base)) (/ Health MaxHealth)))

(event `self.BP_OnManaChanged`
  (params (Mana :type "Float (single-precision)") (MaxMana :type "Float (single-precision)"))
  ;[1 1 1] UI
  (bind _asbp_player_controller_base (cast `/Game/BluePrint/BP_PlayerControllerBase` (`self.GetController`)))
  (`/Game/UI/WBP_HealthBar.SetPercentage` (`/Game/UI/WBP_PrimaryUI.WBP_ManaBar` (`/Game/BluePrint/BP_PlayerControllerBase.Primary UI` _asbp_player_controller_base)) (/ Mana MaxMana)))

(fn `UserConstructionScript`
  (`parent.UserConstructionScript`))