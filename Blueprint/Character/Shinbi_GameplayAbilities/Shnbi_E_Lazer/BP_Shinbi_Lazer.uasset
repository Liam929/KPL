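; Laser actor for Shinbi's E ability that tracks hostile characters in its LazerEnd component and periodically reports them for damage.
; Overlap events maintain a target array, using the instigator's hostility check to admit characters.
; A looping half-second timer sends the array as target data in a Skill.lazer.dealDamage gameplay event to the instigator, so the actor applies no damage itself.
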(event `self.LazerEnd.OnComponentBeginOverlap`
  (params (OverlappedComponent :type "PrimitiveComponent Object Reference") (OtherActor :type "Actor Object Reference") (OtherComp :type "PrimitiveComponent Object Reference") (OtherBodyIndex :type Integer) (bFromSweep :type Boolean) (SweepResult :type "HitResult Structure (by ref)"))
  (bind _asbp_shinbi_character_base (cast `/Game/BluePrint/Character/BP_Shinbi_CharacterBase` OtherActor))
  (bind _asbp_shinbi_character_base_2 (cast `/Game/BluePrint/Character/BP_Shinbi_CharacterBase` (`self.GetInstigator`)))
  (bind _returnvalue (`wzryCharacter.IsOtherHostile` _asbp_shinbi_character_base_2 _asbp_shinbi_character_base))
  (if _returnvalue
    (`KismetArrayLibrary.Array_AddUnique` (`self.OverlapActor`) _asbp_shinbi_character_base)))

(event `self.LazerEnd.OnComponentEndOverlap`
  (params (OverlappedComponent :type "PrimitiveComponent Object Reference") (OtherActor :type "Actor Object Reference") (OtherComp :type "PrimitiveComponent Object Reference") (OtherBodyIndex :type Integer))
  (bind _asbp_shinbi_character_base (cast `/Game/BluePrint/Character/BP_Shinbi_CharacterBase` OtherActor))
  (`KismetArrayLibrary.Array_RemoveItem` (`self.OverlapActor`) _asbp_shinbi_character_base))

(event `self.ReceiveBeginPlay`
  ;[1 1 1] Send Damage Event per 0.5s
  (`KismetSystemLibrary.K2_SetTimerDelegate` (delegate `SendDealDamageEvent`) 0.5 true))

(event `SendDealDamageEvent`
  ;[1 1 1] Send Damage Event per 0.5s
  (if (`KismetMathLibrary.Conv_IntToBool` (`KismetArrayLibrary.Array_Length` (`self.OverlapActor`)))
    (`AbilitySystemBlueprintLibrary.SendGameplayEventToActor` (`self.GetInstigator`) (struct :`TagName` "skill.lazer.dealDamage") (make `GameplayEventData` (struct) null null null null (struct) (struct) (struct) 0.0 (`AbilitySystemBlueprintLibrary.AbilityTargetDataFromActorArray` (`self.OverlapActor`))))))

(fn `UserConstructionScript`)