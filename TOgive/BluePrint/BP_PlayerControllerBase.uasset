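; Player controller for cursor-driven click-to-move play with melee combat and abilities, which creates the primary HUD on BeginPlay.
; Holding SetDestination opens a Tick gate that moves toward the cursor hit; pressing it on a nearby Enemy-tagged actor also triggers melee, with movement zeroed around the call.
; PrimaryAttack calls melee directly.
; Four slot inputs look up the ability class in the HUD and activate it through the pawn's Ability System Component.
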(event `self.AddAbilityToUI`
  (params (AbilityInfo :type "GameplayAbilityInfo Structure"))
  (`/Game/UI/WBP_PrimaryUI.AddAbilityToSlot` (`self.Primary UI`) AbilityInfo))

(event `self.ReceiveBeginPlay`
  ;[1 1 1] Add UI on Screen
  (bind _returnvalue (`|CreateWidget` "/Game/UI/WBP_PrimaryUI.WBP_PrimaryUI_C"))
  (bind _output_get (set `self.Primary UI` _returnvalue))
  (`UserWidget.AddToViewport` _output_get 0))

(event `InputAction|SetDestination`
  (params (Key :type "Key Structure"))
  (bind _returnvalue (`self.K2_GetPawn`))
  (bind (_bblockinghit _binitialoverlap _time _distance _location _impactpoint _normal _impactnormal _physmat _hitactor) (`GameplayStatics.BreakHitResult` (`self.GetHitResultUnderCursorByChannel` "TraceTypeQuery2")))
  ;[1 1 1] 注释
  (:`Pressed`
    (if (<= (`KismetMathLibrary.VSize` (- (`self.K2_GetActorLocation` (`self.K2_GetPawn`)) _location)) 300.0)
      (if (`self.ActorHasTag` _hitactor (`self.Enemy`))
        (bind _asbp_character_base (cast `/Game/BluePrint/Character_Yin/BP_CharacterBase` _returnvalue))
        (bind _charactermovement (`Character.CharacterMovement` _asbp_character_base))
        (set `CharacterMovementComponent.MaxWalkSpeed` 0.0 _charactermovement)
        (set `CharacterMovementComponent.RotationRate` (struct) _charactermovement)
        (`/Game/BluePrint/Character_Yin/BP_CharacterBase.Melee_Attack` _asbp_character_base)
        (bind _asbp_character_base_2 (cast `/Game/BluePrint/Character_Yin/BP_CharacterBase` _returnvalue))
        (bind _charactermovement_2 (`Character.CharacterMovement` _asbp_character_base_2))
        (set `CharacterMovementComponent.MaxWalkSpeed` 600.0 _charactermovement_2)
        (set `CharacterMovementComponent.RotationRate` (struct :`Yaw` 950.0) _charactermovement_2)))))

(event `self.ReceiveTick`
  (params (DeltaSeconds :type "Float (single-precision)"))
  ;[1 1 1] Move to Location
  (`/Engine/EditorBlueprintResources/StandardMacros.Gate` true :!label _label
    (:`Exit`
      (`self.Move To Location` (`self.GetHitResultUnderCursorByChannel` "TraceTypeQuery2")))))

(event `InputAction|SetDestination`
  (params (Key :type "Key Structure"))
  ;[1 1 1] Move to Location
  (:`Pressed`
    (goto _label :!via `Open`))
  (:`Released`
    (goto _label :!via `Close`)))

(event `InputAction|PrimaryAttack`
  (params (Key :type "Key Structure"))
  (:`Pressed`
    (bind _asbp_character_base (cast `/Game/BluePrint/Character_Yin/BP_CharacterBase` (`self.K2_GetPawn`)))
    (`/Game/BluePrint/Character_Yin/BP_CharacterBase.Melee_Attack` _asbp_character_base)))

(event `InputAction|SlotOneAbility`
  (params (Key :type "Key Structure"))
  (:`Pressed`
    (`self.TryActivateAbilityInUISlot` 0)))

(event `InputAction|SlotTwoAbility`
  (params (Key :type "Key Structure"))
  (:`Pressed`
    (`self.TryActivateAbilityInUISlot` 1)))

(event `InputAction|SlotThreeAbility`
  (params (Key :type "Key Structure"))
  (:`Pressed`
    (`self.TryActivateAbilityInUISlot` 2)))

(event `InputAction|SlotFourAbility`
  (params (Key :type "Key Structure"))
  (:`Pressed`
    (`self.TryActivateAbilityInUISlot` 3)))

(fn `Move To Location`
  (params (`Hit Result` :type "HitResult Structure"))
  (`AIBlueprintHelperLibrary.SimpleMoveToLocation` self (`.Location` (`GameplayStatics.BreakHitResult` `Hit Result`))))

(fn `TryActivateAbilityInUISlot`
  (params (SlotNumber :type Integer))
  (bind (_abilityclass _valid) (`/Game/UI/WBP_PrimaryUI.GetSlotAbilityClass` (`self.Primary UI`) SlotNumber))
  (if _valid
    (bind _asbp_character_base (cast `/Game/BluePrint/Character_Yin/BP_CharacterBase` (`self.K2_GetPawn`)))
    (`AbilitySystemComponent.TryActivateAbilityByClass` (`AbilitySystemBlueprintLibrary.GetAbilitySystemComponent` _asbp_character_base) _abilityclass true)))

(fn `UserConstructionScript`)