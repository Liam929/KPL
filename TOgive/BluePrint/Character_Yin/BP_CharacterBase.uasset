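; Base character Blueprint built on the Gameplay Ability System, handling combat hits, health bar updates and montage-driven death.
; BeginPlay grants initial abilities and applies a regen effect, while Melee_Attack activates the melee ability.
; Sword and capsule overlaps with hostile characters send gameplay events for melee and dash damage, with an exclusion list preventing repeat dash hits.
; PushCharacter briefly zeroes ground friction for knockback with optional hit stun.
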(event `self.ReceiveBeginPlay`
  ;[1 1 1] 注释
  (`self.AcquireAbilities` (`self.Initial Ability`))
  (`AbilitySystemComponent.BP_ApplyGameplayEffectToSelf` :`self` (`self.AbilitySystemcomp`) :`GameplayEffectClass` "/Game/BluePrint/Character_Yin/GameplayAbility/GeneralGameplayEffect/GE_BasicRegen.GE_BasicRegen_C"))

(event `TryHealthRegen`
  ;[1 1 1] 注释
)

(event `Melee_Attack`
  ;[1 1 1] 注释
  (`AbilitySystemComponent.TryActivateAbilityByClass` (`self.AbilitySystemcomp`) "/Game/BluePrint/Character_Yin/GameplayAbility/Melee/GA_Melee.GA_Melee_C" true))

(event `TryDash`
  ;[1 1 1] 注释
)

(event `MakeCameraControlRotation`
  (params (should :type Boolean))
  (if should
    (set `self.bUseControllerRotationYaw` true)
    (set `CharacterMovementComponent.bOrientRotationToMovement` false (`self.CharacterMovement`))
    (else
      (set `self.bUseControllerRotationYaw` false)
      (set `CharacterMovementComponent.bOrientRotationToMovement` true (`self.CharacterMovement`)))))

(event `self.ReceiveTick`
  (params (DeltaSeconds :type "Float (single-precision)"))
  ;[1 1 1] 注释
)

(event `self.SwordCollider.OnComponentBeginOverlap`
  (params (OverlappedComponent :type "PrimitiveComponent Object Reference") (OtherActor :type "Actor Object Reference") (OtherComp :type "PrimitiveComponent Object Reference") (OtherBodyIndex :type Integer) (bFromSweep :type Boolean) (SweepResult :type "HitResult Structure (by ref)"))
  ;[1 1 1] 注释
  (if (!= OtherActor self)
    (bind _asbp_character_base (cast `/Game/BluePrint/Character_Yin/BP_CharacterBase` OtherActor))
    (bind _returnvalue (`self.IsOtherHostile` _asbp_character_base self))
    (if _returnvalue
      (`AbilitySystemBlueprintLibrary.SendGameplayEventToActor` self (struct :`TagName` "Skill.Melee.DealDamage") (make `GameplayEventData` (struct) null OtherActor)))))

(event `self.BP_Die`
  ;[1 1 1] 注释
  (bind _returnvalue (`self.PlayAnimMontage` "/Game/BluePrint/Character_Yin/Animation/Death_Montage.Death_Montage"))
  (`KismetSystemLibrary.Delay` _returnvalue)
  (`self.K2_DestroyActor`))

(event `self.BP_OnHealthChanged`
  (params (Health :type "Float (single-precision)") (MaxHealth :type "Float (single-precision)"))
  ;[1 1 1] 血条显示
  (bind _ashealth_bar (cast `/Game/UI/HealthBar` (`WidgetComponent.GetUserWidgetObject` (`self.HealthBar`))))
  (`/Game/UI/HealthBar.SetPercentage` _ashealth_bar (/ Health MaxHealth)))

(event `self.CapsuleComponent.OnComponentBeginOverlap`
  (params (OverlappedComponent :type "PrimitiveComponent Object Reference") (OtherActor :type "Actor Object Reference") (OtherComp :type "PrimitiveComponent Object Reference") (OtherBodyIndex :type Integer) (bFromSweep :type Boolean) (SweepResult :type "HitResult Structure (by ref)"))
  (bind _asbp_character_base (cast `/Game/BluePrint/Character_Yin/BP_CharacterBase` OtherActor))
  (bind _returnvalue (`self.IsOtherHostile` _asbp_character_base self))
  (if _returnvalue
    (if (not (`KismetArrayLibrary.Array_Contains` (`self.OverLapExculde`) _asbp_character_base))
      (`KismetArrayLibrary.Array_AddUnique` (`self.OverLapExculde`) _asbp_character_base)
      (`AbilitySystemBlueprintLibrary.SendGameplayEventToActor` self (struct :`TagName` "skill.Dash.Dealdamage") (make `GameplayEventData` (struct) self OtherActor)))))

(event `PushCharacter`
  (params (ImpulseDirection :type "Vector Structure") (PushStrength :type "Float (double-precision)") (StunDuration :type "Float (double-precision)"))
  (bind _charactermovement (`self.CharacterMovement`))
  (set `self.DeafaultGroundFriction` (`CharacterMovementComponent.GroundFriction` _charactermovement))
  (set `CharacterMovementComponent.GroundFriction` 0.0 _charactermovement)
  (`CharacterMovementComponent.AddImpulse` (`self.CharacterMovement`) (* ImpulseDirection PushStrength) true)
  (if (> StunDuration 0.0)
    (`self.HitStun` StunDuration))
  (`KismetSystemLibrary.Delay` 0.3)
  (set `CharacterMovementComponent.GroundFriction` (`self.DeafaultGroundFriction`) (`self.CharacterMovement`)))

(fn `SetCollisonToPawn`
  (params (NewResponse :type "ECollisionResponse Enum" :default "ECR_Ignore"))
  (`PrimitiveComponent.SetCollisionResponseToChannel` (`self.CapsuleComponent`) "ECC_Pawn" NewResponse))

(fn `UserConstructionScript`)