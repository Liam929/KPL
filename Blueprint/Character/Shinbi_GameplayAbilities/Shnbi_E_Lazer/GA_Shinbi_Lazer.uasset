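; Shinbi's E-slot laser Gameplay Ability, a timed beam that deals damage while its cost can be paid.
; It plays a montage, then after a short delay attaches a laser actor to the mesh socket and enables mouse-controlled rotation.
; Gameplay events trigger damage on target data, ending the ability if cost runs out, otherwise after a delay.
; Ending removes cost-drain effects, destroys the laser and restores rotation.
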(event `self.K2_ActivateAbility`
  (`self.K2_CommitAbility`)
  (`self.DoUICD`)
  (`AbilityTask_PlayMontageAndWait.CreatePlayMontageAndWaitProxy` "None" "/Game/BluePrint/Character/Animation/AM_Shinbi_E_Lazer.AM_Shinbi_E_Lazer"
    (:`then`
      (`KismetSystemLibrary.Delay` 0.3)
      (bind _characterbase (`self.GetCharacterAndController`))
      (bind (_asynctaskproxy _spawnedactor) (`AbilityTask_SpawnActor.SpawnActor` (struct) "/Game/BluePrint/Character/Shinbi_GameplayAbilities/Shnbi_E_Lazer/BP_Shinbi_Lazer.BP_Shinbi_Lazer_C" _characterbase)
        (:`then`
          (bind _output_get (set `self.LazerActor` _spawnedactor))
          (`Actor.K2_AttachToComponent` _output_get (`Character.Mesh` _characterbase) "Lazer" "SnapToTarget" "SnapToTarget" "KeepRelative" true)
          (`/Game/BluePrint/Character/BP_Shinbi_CharacterBase.MakeMouseControlRotation` _characterbase true)
          (bind (_asynctaskproxy_2 _payload) (`AbilityTask_WaitGameplayEvent.WaitGameplayEvent` (struct :`TagName` "skill.lazer.dealDamage") null)
            (:`then`
              (`KismetSystemLibrary.Delay` 3.0)
              (`self.K2_EndAbility`))
            (:`EventReceived`
              (bind _can (`self.IsCostStillAvaliable`))
              (if _can
                (`self.BP_ApplyGameplayEffectToTarget` (`.TargetData` (break `GameplayEventData` _payload)) "/Game/BluePrint/Character/Shinbi_GameplayAbilities/Shnbi_E_Lazer/GE_Shinbi_Lazer_Damage.GE_Shinbi_Lazer_Damage_C")
                (`KismetSystemLibrary.Delay` 3.0)
                (`self.K2_EndAbility`)
                (else
                  (`self.K2_EndAbility`))))))))))

(event `self.K2_OnEndAbility`
  (params (bWasCancelled :type Boolean))
  (`self.BP_RemoveGameplayEffectFromOwnerWithAssetTags` (struct :`GameplayTags` (struct :`(TagName` "skill.lazer.drainingCost"))))
  (`Actor.K2_DestroyActor` (`self.LazerActor`))
  (bind _characterbase (`self.GetCharacterAndController`))
  (`/Game/BluePrint/Character/BP_Shinbi_CharacterBase.MakeMouseControlRotation` _characterbase false))