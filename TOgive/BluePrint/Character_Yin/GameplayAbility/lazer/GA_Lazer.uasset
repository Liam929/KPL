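; Gameplay ability for a laser skill that damages and briefly stuns targets while its cost remains affordable.
; Activation commits, plays the casting montage, attaches a spawned BP_Lazer to the caster's mesh socket and sets camera-controlled rotation.
; Skill.Lazer.Damage events supply target data for the damage effect and a zero-impulse PushCharacter stun, or end the ability when cost runs out.
; Montage exit also ends it, removing the draining-cost effect and destroying the laser.
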(event `self.K2_ActivateAbility`
  (`self.K2_CommitAbility`)
  (`self.DOUICoollDown`)
  (`AbilityTask_PlayMontageAndWait.CreatePlayMontageAndWaitProxy` "None" "/Game/BluePrint/Character_Yin/Animation/AM_LazerCasting.AM_LazerCasting"
    (:`then`
      (`KismetSystemLibrary.Delay` 0.0)
      (bind _charabase (`self.GetPlayerInfo`))
      (bind (_asynctaskproxy _spawnedactor) (`AbilityTask_SpawnActor.SpawnActor` (struct) "/Game/BluePrint/Character_Yin/GameplayAbility/lazer/BP_Lazer.BP_Lazer_C" _charabase)
        (:`then`
          (bind _output_get (set `self.LazerActor` _spawnedactor))
          (`Actor.K2_AttachToComponent` _output_get (`Character.Mesh` _charabase) "Lazer" "SnapToTarget" "SnapToTarget" "KeepRelative" true)
          (`/Game/BluePrint/Character_Yin/BP_CharacterBase.MakeCameraControlRotation` _charabase true)
          (bind (_asynctaskproxy_2 _payload) (`AbilityTask_WaitGameplayEvent.WaitGameplayEvent` (struct :`TagName` "skill.Lazer.Damage") null)
            (:`EventReceived`
              (bind _can (`self.IsCosrStillAvaluable`))
              (if _can
                (bind (_eventtag _instigator _target _optionalobject _optionalobject2 _contexthandle _instigatortags _targettags _eventmagnitude _targetdata) (break `GameplayEventData` _payload))
                (`self.BP_ApplyGameplayEffectToTarget` _targetdata "/Game/BluePrint/Character_Yin/GameplayAbility/lazer/GE_LazerDamage.GE_LazerDamage_C")
                (for _array_element (`AbilitySystemBlueprintLibrary.GetActorsFromTargetData` _targetdata)
                  (bind _asbp_character_base (cast `/Game/BluePrint/Character_Yin/BP_CharacterBase` _array_element))
                  (`/Game/BluePrint/Character_Yin/BP_CharacterBase.PushCharacter` _asbp_character_base (0.0 0.0 0.0) 0.0 0.3))
                (else
                  (`self.K2_EndAbility`))))))))
    (:`OnCompleted`
      (`self.K2_EndAbility` :!label _label))
    (:`OnBlendOut`
      (goto _label))
    (:`OnInterrupted`
      (goto _label))
    (:`OnCancelled`
      (goto _label))))

(event `self.K2_OnEndAbility`
  (params (bWasCancelled :type Boolean))
  (`self.BP_RemoveGameplayEffectFromOwnerWithAssetTags` (struct :`GameplayTags` (struct :`(TagName` "skill.Lazer.draningcost"))))
  (`Actor.K2_DestroyActor` (`self.LazerActor`))
  (bind _charabase (`self.GetPlayerInfo`))
  (`/Game/BluePrint/Character_Yin/BP_CharacterBase.MakeCameraControlRotation` _charabase true))