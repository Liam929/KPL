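; Dash gameplay ability for the Yin character that launches it forward through pawns and knocks up whoever it hits.
; On activation it zeroes ground friction, applies a forward velocity impulse, sets pawn collision to overlap and plays the dash montage.
; Deal-damage gameplay events apply a damage effect to the target and push it upward with a stun.
; When the montage ends or is interrupted, friction and pawn blocking are restored.
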(event `self.K2_ActivateAbility`
  (`self.K2_CommitAbility`)
  (`self.DoUICD`)
  (bind _ascharacter (cast `Character` (`self.GetOwningActorFromActorInfo`))
    (:`then`
      (bind _charactermovement (`Character.CharacterMovement` _ascharacter))
      (set `self.OriginalGroundFriction` (`CharacterMovementComponent.GroundFriction` _charactermovement))
      (set `CharacterMovementComponent.GroundFriction` 0.0 _charactermovement)
      (`CharacterMovementComponent.AddImpulse` _charactermovement (* (`Actor.GetActorForwardVector` _ascharacter) 900.0) true) ; Don't have vector
      (bind _characterbase (`self.GetCharacterAndController`))
      (`/Game/BluePrint/Character/BP_Shinbi_CharacterBase.SetCollisionToPawn` _characterbase "ECR_Overlap")
      (`AbilityTask_PlayMontageAndWait.CreatePlayMontageAndWaitProxy` "None" "/Game/TOGIVE/BluePrint/Character_Yin/Animation/AM_Dash_Yin.AM_Dash_Yin"
        (:`then`
          (bind (_asynctaskproxy _payload) (`AbilityTask_WaitGameplayEvent.WaitGameplayEvent` (struct :`TagName` "skill.dash.dealDamage") null)
            (:`EventReceived`
              (bind (_eventtag _instigator _target) (break `GameplayEventData` _payload))
              (`self.BP_ApplyGameplayEffectToTarget` (`AbilitySystemBlueprintLibrary.AbilityTargetDataFromActor` _target) "/Game/BluePrint/Character/Yin_GameplayAbilities/Dash/GE_DashDamage.GE_DashDamage_C")
              (bind _asbp_shinbi_character_base (cast `/Game/BluePrint/Character/BP_Shinbi_CharacterBase` _target))
              (`/Game/BluePrint/Character/BP_Shinbi_CharacterBase.PushCharacter` _asbp_shinbi_character_base (0.0 0.0 1.0) 600.0 3.0))))
        (:`OnCompleted`
          (set `CharacterMovementComponent.GroundFriction` (`self.OriginalGroundFriction`) _charactermovement :!label _label)
          (bind _characterbase_2 (`self.GetCharacterAndController`))
          (`/Game/BluePrint/Character/BP_Shinbi_CharacterBase.SetCollisionToPawn` _characterbase_2 "ECR_Block")
          (`self.K2_EndAbility`))
        (:`OnBlendOut`
          (goto _label))
        (:`OnInterrupted`
          (goto _label))
        (:`OnCancelled`
          (goto _label))))
    (:`CastFailed`
      (`self.K2_EndAbility`))))