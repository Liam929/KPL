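; BP_Lazer is a laser beam actor for a GAS-based skill that reports which hostile characters it is hitting.
; Overlaps on the Lazerend component maintain a list of BP_CharacterBase targets that the instigator considers hostile.
; A looping timer sends that list as target data in a Skill.Lazer.Damage gameplay event to the instigator, even when empty, rather than applying damage itself.
; Tick only casts the laser mesh's anim instance, with no further effect.
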(event `self.ReceiveBeginPlay`
  (`KismetSystemLibrary.K2_SetTimerDelegate` (delegate `SendDealDamageEvent`) 0.3 true))

(event `SendDealDamageEvent`
  (if (`KismetMathLibrary.Conv_IntToBool` (`KismetArrayLibrary.Array_Length` (`self.OverlapingActor`)))
    _
    (else
      _))
  (`AbilitySystemBlueprintLibrary.SendGameplayEventToActor` (`self.GetInstigator`) (struct :`TagName` "skill.Lazer.Damage") (make `GameplayEventData` (struct :`TagName` "skill.Lazer.Damage") null null null null (struct) (struct) (struct) 0.0 (`AbilitySystemBlueprintLibrary.AbilityTargetDataFromActorArray` (`self.OverlapingActor`)))))

(event `self.ReceiveTick`
  (params (DeltaSeconds :type "Float (single-precision)"))
  (cast `/Game/BluePrint/Character_Yin/GameplayAbility/lazer/LazerAssets/Animation_BPlazer_skeletal_mesh_Skeleton` (`SkeletalMeshComponent.GetAnimInstance` (`self.LazerMesh`))))

(event `self.Lazerend.OnComponentBeginOverlap`
  (params (OverlappedComponent :type "PrimitiveComponent Object Reference") (OtherActor :type "Actor Object Reference") (OtherComp :type "PrimitiveComponent Object Reference") (OtherBodyIndex :type Integer) (bFromSweep :type Boolean) (SweepResult :type "HitResult Structure (by ref)"))
  (bind _asbp_character_base (cast `/Game/BluePrint/Character_Yin/BP_CharacterBase` OtherActor))
  (bind _asbp_character_base_2 (cast `/Game/BluePrint/Character_Yin/BP_CharacterBase` (`self.GetInstigator`)))
  (bind _returnvalue (`MyCharacterBase.IsOtherHostile` _asbp_character_base_2 _asbp_character_base))
  (if _returnvalue
    (`KismetArrayLibrary.Array_AddUnique` (`self.OverlapingActor`) _asbp_character_base)))

(event `self.Lazerend.OnComponentEndOverlap`
  (params (OverlappedComponent :type "PrimitiveComponent Object Reference") (OtherActor :type "Actor Object Reference") (OtherComp :type "PrimitiveComponent Object Reference") (OtherBodyIndex :type Integer))
  (bind _asbp_character_base (cast `/Game/BluePrint/Character_Yin/BP_CharacterBase` OtherActor))
  (`KismetArrayLibrary.Array_RemoveItem` (`self.OverlapingActor`) _asbp_character_base))

(fn `UserConstructionScript`)