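; Player character Blueprint for Shinbi that links attribute changes to the HUD and handles death and respawn.
; Health and mana change events set percentage bars on the PrimaryUI owned by BP_PlayerControllerBase.
; Die waits out the death montage, applies a death-increment GameplayEffect, then resets the actor to DefaultTransform.
; It then applies a respawn GameplayEffect through the Ability System Component and calls Respawn.
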(event `self.BP_OnHealthChanged`
  (params (Health :type "Float (single-precision)") (MaxHealth :type "Float (single-precision)"))
  ;[1 1 1] Set Health Bar
  (bind _asbp_player_controller_base (cast `/Game/BluePrint/Character/BP_PlayerControllerBase` (`self.GetController`)))
  (`ProgressBar.SetPercent` (`/Game/UI/WidgetBP/WBP_PrimaryUI.HealthBar` (`/Game/BluePrint/Character/BP_PlayerControllerBase.PrimaryUI` _asbp_player_controller_base)) (/ Health MaxHealth)))

(event `self.BP_OnManaChanged`
  (params (Mana :type "Float (single-precision)") (MaxMana :type "Float (single-precision)"))
  ;[1 1 1] Set Mana Bar
  (bind _asbp_player_controller_base (cast `/Game/BluePrint/Character/BP_PlayerControllerBase` (`self.GetController`)))
  (`ProgressBar.SetPercent` (`/Game/UI/WidgetBP/WBP_PrimaryUI.ManaBar` (`/Game/BluePrint/Character/BP_PlayerControllerBase.PrimaryUI` _asbp_player_controller_base)) (/ Mana MaxMana)))

(event `self.BP_Die`
  ;[1 1 1] Die Event
  (bind _returnvalue (`self.PlayAnimMontage` "/Game/BluePrint/Character/Animation/AM_Shinbi_Die.AM_Shinbi_Die"))
  (`KismetSystemLibrary.Delay` _returnvalue)
  (`AbilitySystemComponent.BP_ApplyGameplayEffectToSelf` :`self` (`self.AbilitySystemComp`) :`GameplayEffectClass` "/Game/BluePrint/Character/Shinbi_GameplayAbilities/GameplayEffect/IncreaseEffect/GE_IncreaseDeath.GE_IncreaseDeath_C")
  (`self.K2_SetActorRelativeTransform` (`self.DefaultTransform`))
  (`AbilitySystemComponent.BP_ApplyGameplayEffectToSelf` :`self` (`self.AbilitySystemComp`) :`GameplayEffectClass` "/Game/BluePrint/Character/Shinbi_GameplayAbilities/GameplayEffect/IncreaseEffect/GE_Respawn.GE_Respawn_C")
  (`self.Respawn`))

(fn `UserConstructionScript`
  (`parent.UserConstructionScript`))