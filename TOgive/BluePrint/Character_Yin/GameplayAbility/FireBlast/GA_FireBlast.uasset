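; Gameplay ability for the Fire Blast skill: a two-stage pull and push on characters around the caster, with damage.
; It commits, starts the UI cooldown and plays a montage whose pull event triggers instant radius targeting and a first impulse with stun.
; The push event damages those stored targets and applies a stronger, opposite impulse, its direction computed from the first loop's character reference.
; The ability ends with the montage.
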(event `self.K2_ActivateAbility`
  (bind _targetdatahandle (`self.TargetDataHandle`))
  (`self.K2_CommitAbility`)
  (`self.DOUICoollDown`)
  (`AbilityTask_PlayMontageAndWait.CreatePlayMontageAndWaitProxy` "None" "/Game/BluePrint/Character_Yin/Animation/AM_FireBlast.AM_FireBlast"
    (:`then`
      (`AbilityTask_WaitGameplayEvent.WaitGameplayEvent` (struct :`TagName` "skill.FireBlast.pull") null
        (:`EventReceived`
          (bind (_asynctaskproxy _data) (`AbilityTask_WaitTargetData.WaitTargetData` "None" "Instant" "/Script/LOL_TEST2.GATargetActorGetAround" 300.0 (struct) (struct) null)
            (:`then`
              (`AbilityTask_WaitGameplayEvent.WaitGameplayEvent` (struct :`TagName` "skill.FireBlast.push") null
                (:`EventReceived`
                  (`self.BP_ApplyGameplayEffectToTarget` _targetdatahandle "/Game/BluePrint/Character_Yin/GameplayAbility/FireBlast/GE_FireBlastDAmage.GE_FireBlastDAmage_C")
                  (for _array_element (`AbilitySystemBlueprintLibrary.GetActorsFromTargetData` _targetdatahandle)
                    (bind _asbp_character_base (cast `/Game/BluePrint/Character_Yin/BP_CharacterBase` _array_element))
                    (bind _returnvalue (`KismetMathLibrary.Normal` (- (`Actor.K2_GetActorLocation` (stale _asbp_character_base_2)) (`Actor.K2_GetActorLocation` (`self.GetOwningActorFromActorInfo`)))))
                    (`/Game/BluePrint/Character_Yin/BP_CharacterBase.PushCharacter` _asbp_character_base (* _returnvalue -1.0) 2000.0 2.0)))))
            (:`ValidData`
              (set `self.TargetDataHandle` _data)
              (for _array_element_2 (`AbilitySystemBlueprintLibrary.GetActorsFromTargetData` _data)
                (bind _asbp_character_base_2 (cast `/Game/BluePrint/Character_Yin/BP_CharacterBase` _array_element_2))
                (`/Game/BluePrint/Character_Yin/BP_CharacterBase.PushCharacter` _asbp_character_base_2 _returnvalue 800.0 1.0)))))))
    (:`OnCompleted`
      (`self.K2_EndAbility` :!label _label))
    (:`OnBlendOut`
      (goto _label))
    (:`OnInterrupted`
      (goto _label))
    (:`OnCancelled`
      (goto _label))))