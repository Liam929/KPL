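; Player controller for click-to-move, mouse-driven combat with the Shinbi character, which also creates the primary UI.
; Holding SetDestination moves the pawn toward the cursor hit through a gated Tick; pressing it on a nearby Enemy-tagged actor attacks, briefly freezing movement and rotation.
; Q/W/E/R skills activate Gameplay Ability System abilities looked up from UI slots, setting the targeting state for target-type abilities.
; Separate inputs forward target selection and cancellation.
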(event `self.ReceiveTick`
  (params (DeltaSeconds :type "Float (single-precision)"))
  ;[1 1 1] Move To Location
  (`/Engine/EditorBlueprintResources/StandardMacros.Gate` true :!label _label
    (:`Exit`
      (`self.MoveToLocation` (`self.GetHitResultUnderCursorByChannel` "TraceTypeQuery2")))))

(event `InputAction|SetDestination`
  (params (Key :type "Key Structure"))
  ;[1 1 1] Move To Location
  (:`Pressed`
    (goto _label :!via `Open`))
  (:`Released`
    (goto _label :!via `Close`)))

(event `self.ReceiveBeginPlay`
  ;[1 1 1] Add UI on Screen
  (bind _returnvalue (`|CreateWidget` "/Game/UI/WidgetBP/WBP_PrimaryUI.WBP_PrimaryUI_C"))
  (bind _output_get (set `self.PrimaryUI` _returnvalue))
  (`UserWidget.AddToViewport` _output_get 0))

(event `InputAction|SetDestination`
  (params (Key :type "Key Structure"))
  (bind _returnvalue (`self.K2_GetPawn`))
  (bind (_bblockinghit _binitialoverlap _time _distance _location _impactpoint _normal _impactnormal _physmat _hitactor) (`GameplayStatics.BreakHitResult` (`self.GetHitResultUnderCursorByChannel` "TraceTypeQuery2")))
  ;[1 1 1] Use Mouse To Attack
  (:`Pressed`
    (if (<= (`KismetMathLibrary.VSize` (- (`self.K2_GetActorLocation` (`self.K2_GetPawn`)) _location)) 150.0)
      (if (`self.ActorHasTag` _hitactor (`self.Enemy`))
        (bind _asbp_shinbi_character_base (cast `/Game/BluePrint/Character/BP_Shinbi_CharacterBase` _returnvalue))
        (bind _charactermovement (`Character.CharacterMovement` _asbp_shinbi_character_base))
        (set `CharacterMovementComponent.MaxWalkSpeed` 0.0 _charactermovement)
        (set `CharacterMovementComponent.RotationRate` (struct) _charactermovement)
        (`/Game/BluePrint/Character/BP_Shinbi_CharacterBase.Attack` _asbp_shinbi_character_base)
        (bind _asbp_shinbi_character_base_2 (cast `/Game/BluePrint/Character/BP_Shinbi_CharacterBase` _returnvalue))
        (`KismetSystemLibrary.Delay` 0.6)
        (bind _charactermovement_2 (`Character.CharacterMovement` _asbp_shinbi_character_base_2))
        (set `CharacterMovementComponent.MaxWalkSpeed` 600.0 _charactermovement_2)
        (set `CharacterMovementComponent.RotationRate` (struct :`Yaw` 950.0) _charactermovement_2)))))

(event `InputAction|TargetSelect`
  (params (Key :type "Key Structure"))
  ;[1 1 1] Use Mouse To Select Target
  (:`Pressed`
    (bind _asbp_shinbi_character_base (cast `/Game/BluePrint/Character/BP_Shinbi_CharacterBase` (`self.K2_GetPawn`)))
    (`/Game/BluePrint/Character/BP_Shinbi_CharacterBase.TargetSelect` _asbp_shinbi_character_base)))

(event `InputAction|InputActionCancel`
  (params (Key :type "Key Structure"))
  ;[1 1 1] Use Mouse To Cancel Target Select
  (:`Pressed`
    (bind _asbp_shinbi_character_base (cast `/Game/BluePrint/Character/BP_Shinbi_CharacterBase` (`self.K2_GetPawn`)))
    (`AbilitySystemComponent.TargetCancel` (`AbilitySystemBlueprintLibrary.GetAbilitySystemComponent` _asbp_shinbi_character_base))))

(event `InputAction|SkillQ`
  (params (Key :type "Key Structure"))
  ;[1 1 1] Skill Q Dash
  (:`Pressed`
    (`self.TryActivateAbilityInUISlot` 0)))

(event `InputAction|SkillE`
  (params (Key :type "Key Structure"))
  ;[1 1 1] Skill E Lazer
  (:`Pressed`
    (`self.TryActivateAbilityInUISlot` 2)))

(event `InputAction|SkillW`
  (params (Key :type "Key Structure"))
  ;[1 1 1] Skill W Health Regen
  (:`Pressed`
    (`self.TryActivateAbilityInUISlot` 1)))

(event `InputAction|SkillR`
  (params (Key :type "Key Structure"))
  ;[1 1 1] Skill E Lazer
  (:`Pressed`
    (`self.TryActivateAbilityInUISlot` 3)))

(event `self.AddAbilityToUI`
  (params (AbilityInfo :type "GameplayAbilityInfo Structure"))
  ;[1 1 1] Add Ability To UI
  (`/Game/UI/WidgetBP/WBP_PrimaryUI.AddAbilityToSlots` (`self.PrimaryUI`) AbilityInfo))

(fn `MoveToLocation`
  (params (HitResult :type "HitResult Structure"))
  (`AIBlueprintHelperLibrary.SimpleMoveToLocation` self (`.Location` (`GameplayStatics.BreakHitResult` HitResult))))

(fn `TryActivateAbilityInUISlot`
  (params (SlotNum :type Integer))
  (bind (_gameplayability _valid) (`/Game/UI/WidgetBP/WBP_PrimaryUI.GetSlotAbilityClass` (`self.PrimaryUI`) SlotNum))
  (if _valid
    (bind _asbp_shinbi_character_base (cast `/Game/BluePrint/Character/BP_Shinbi_CharacterBase` (`self.K2_GetPawn`)))
    (`AbilitySystemComponent.TryActivateAbilityByClass` (`AbilitySystemBlueprintLibrary.GetAbilitySystemComponent` _asbp_shinbi_character_base) _gameplayability true)
    (castclass `/Game/BluePrint/Character/Shinbi_GameplayAbilities/BP_Shinbi_GameplayAbility_Target` _gameplayability
      (:`then`
        (set `/Game/BluePrint/Character/BP_Shinbi_CharacterBase.Targeting` true _asbp_shinbi_character_base))
      (:`CastFailed`
        (set `/Game/BluePrint/Character/BP_Shinbi_CharacterBase.Targeting` false _asbp_shinbi_character_base)
        (`AbilitySystemComponent.TargetCancel` (`AbilitySystemBlueprintLibrary.GetAbilitySystemComponent` _asbp_shinbi_character_base))))))

(fn `UserConstructionScript`)