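; Gameplay ability for Yin's dash: launches the character forward with a velocity impulse, passing through pawns and damaging those it hits.
; On activation it commits, triggers the UI cooldown, zeroes ground friction, sets pawn collision to overlap and plays the dash montage.
; A damage gameplay event applies the dash damage effect and pushes the target upward with a stun.
; Any montage exit restores friction and blocking collision, then ends the ability.
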(event `self.K2_ActivateAbility`
  (`self.K2_CommitAbility`)
  (`self.DOUICoollDown`)
  (bind _ascharacter (cast `Character` (`self.GetOwningActorFromActorInfo`))
    (:`then`
      (bind _charactermovement (`Character.CharacterMovement` _ascharacter))
      (set `self.Original Ground Friction` (`CharacterMovementComponent.GroundFriction` _charactermovement))
      (set `CharacterMovementComponent.GroundFriction` 0.0 _charactermovement)
      (`CharacterMovementComponent.AddImpulse` _charactermovement (* (`Actor.GetActorForwardVector` _ascharacter) 1000.0) true)
      (bind _charabase (`self.GetPlayerInfo`))
      (`/Game/BluePrint/Character_Yin/BP_CharacterBase.SetCollisonToPawn` _charabase "ECR_Overlap")
      (`AbilityTask_PlayMontageAndWait.CreatePlayMontageAndWaitProxy` "None" "/Game/BluePrint/Character_Yin/Animation/AM_Dash_Yin.AM_Dash_Yin"
        (:`then`
          (bind (_asynctaskproxy _payload) (`AbilityTask_WaitGameplayEvent.WaitGameplayEvent` (struct :`TagName` "skill.Dash.Dealdamage") null)
            (:`EventReceived`
              (bind (_eventtag _instigator _target) (break `GameplayEventData` _payload))
              (`self.BP_ApplyGameplayEffectToTarget` (`AbilitySystemBlueprintLibrary.AbilityTargetDataFromActor` _target) "/Game/BluePrint/Character_Yin/GameplayAbility/Dash/GE_DashDamage.GE_DashDamage_C")
              (bind _asbp_character_base (cast `/Game/BluePrint/Character_Yin/BP_CharacterBase` _target))
              (`/Game/BluePrint/Character_Yin/BP_CharacterBase.PushCharacter` _asbp_character_base (0.0 0.0 1.0) 600.0 3.0))))
        (:`OnCompleted`
          (set `CharacterMovementComponent.GroundFriction` (`self.Original Ground Friction`) _charactermovement :!label _label)
          (bind _charabase_2 (`self.GetPlayerInfo`))
          (`/Game/BluePrint/Character_Yin/BP_CharacterBase.SetCollisonToPawn` _charabase_2 "ECR_Block")
          (`self.K2_EndAbility`))
        (:`OnBlendOut`
          (goto _label))
        (:`OnInterrupted`
          (goto _label))
        (:`OnCancelled`
          (goto _label))))
    (:`CastFailed`
      (`self.K2_EndAbility`))))