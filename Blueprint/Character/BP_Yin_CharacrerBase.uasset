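; Base player character Blueprint built on the Gameplay Ability System, handling startup abilities, HUD bars and respawning.
; BeginPlay grants initial abilities, applies level-scaled regen and level effects, and caches the spawn transform and tagged enemy count.
; Health and mana events update the player controller's UI, while another event toggles camera-driven rotation.
; Death plays a montage, applies death-count and respawn effects, restores the saved transform and calls Respawn.
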(event `self.ReceiveBeginPlay`
  (bind (_level_basevalue _level_currentvalue) (break `GameplayAttributeData` (`AttributeSetBase.Level` (`self.AttributeSetBaseComp`))))
  (bind (_level_basevalue_2 _level_currentvalue_2) (break `GameplayAttributeData` (`AttributeSetBase.Level` (`self.AttributeSetBaseComp`))))
  ;[1 1 1] Acquire Abilities
  (`self.AcquireAbilities` (`self.InitialAbilities`))
  ;[1 1 1] Get Enemy Number
  (bind _outactors (`GameplayStatics.GetAllActorsWithTag` (`self.Enemy`)))
  (set `self.DefaultEnemyNumber` (`KismetArrayLibrary.Array_Length` _outactors))
  ;[1 1 1] Level Regen
  (`AbilitySystemComponent.BP_ApplyGameplayEffectToSelf` :`self` (`self.AbilitySystemComp`) :`GameplayEffectClass` "/Game/BluePrint/Character/Shinbi_GameplayAbilities/GameplayEffect/GE_BasicRegen.GE_BasicRegen_C" :`Level` _level_currentvalue_2)
  ;[1 1 1] Level Effect
  (`AbilitySystemComponent.BP_ApplyGameplayEffectToSelf` :`self` (`self.AbilitySystemComp`) :`GameplayEffectClass` "/Game/BluePrint/Character/Shinbi_GameplayAbilities/GameplayEffect/LevelEffect/GE_LevelEffect.GE_LevelEffect_C" :`Level` _level_currentvalue)
  ;[1 1 1] Set Default Transform
  (set `self.DefaultTransform` (`self.GetTransform`)))

(event `self.BP_OnHealthChanged`
  (params (Health :type "Float (single-precision)") (MaxHealth :type "Float (single-precision)"))
  ;[1 1 1] Set Health Bar
  (bind _asbp_player_controller_base (cast `/Game/BluePrint/Character/BP_PlayerControllerBase` (`self.GetController`)))
  (`ProgressBar.SetPercent` (`/Game/UI/WidgetBP/WBP_PrimaryUI.HealthBar` (`/Game/BluePrint/Character/BP_PlayerControllerBase.PrimaryUI` _asbp_player_controller_base)) (/ Health MaxHealth)))

(event `MakeCameraControllRotation`
  (params (Should :type Boolean))
  (if Should
    (set `self.bUseControllerRotationYaw` true)
    (set `CharacterMovementComponent.bOrientRotationToMovement` false (`self.CharacterMovement`))
    (else
      (set `self.bUseControllerRotationYaw` false)
      (set `CharacterMovementComponent.bOrientRotationToMovement` true (`self.CharacterMovement`)))))

(event `self.BP_OnManaChanged`
  (params (Mana :type "Float (single-precision)") (MaxMana :type "Float (single-precision)"))
  ;[1 1 1] Set Mana Bar
  (bind _asbp_player_controller_base (cast `/Game/BluePrint/Character/BP_PlayerControllerBase` (`self.GetController`)))
  (`ProgressBar.SetPercent` (`/Game/UI/WidgetBP/WBP_PrimaryUI.ManaBar` (`/Game/BluePrint/Character/BP_PlayerControllerBase.PrimaryUI` _asbp_player_controller_base)) (/ Mana MaxMana)))

(event `self.BP_Die`
  ;[1 1 1] Die Event
  (bind _returnvalue (`self.PlayAnimMontage` "/Game/TOGIVE/BluePrint/Character_Yin/Animation/Death_Montage.Death_Montage"))
  (`KismetSystemLibrary.Delay` _returnvalue)
  (`AbilitySystemComponent.BP_ApplyGameplayEffectToSelf` :`self` (`self.AbilitySystemComp`) :`GameplayEffectClass` "/Game/BluePrint/Character/Shinbi_GameplayAbilities/GameplayEffect/IncreaseEffect/GE_IncreaseDeath.GE_IncreaseDeath_C")
  (`self.K2_SetActorRelativeTransform` (`self.DefaultTransform`))
  (`AbilitySystemComponent.BP_ApplyGameplayEffectToSelf` :`self` (`self.AbilitySystemComp`) :`GameplayEffectClass` "/Game/BluePrint/Character/Shinbi_GameplayAbilities/GameplayEffect/IncreaseEffect/GE_Respawn.GE_Respawn_C")
  (`self.Respawn`))

(fn `UserConstructionScript`)