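; Enemy character Blueprint that displays its health and handles its own death.
; OnHealthChanged casts the health bar component's widget to WBP_HealthBar and sets its fill from the ratio of current to maximum health.
; Die plays the Shinbi death montage, waits for the duration it returns, then destroys the actor.
; BeginPlay, overlap and Tick events are disabled stubs, so all logic is event-driven.
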(event `self.BP_OnHealthChanged`
  (params (Health :type "Float (single-precision)") (MaxHealth :type "Float (single-precision)"))
  ;[1 1 1] Set Health Bar Percentage
  (bind _aswbp_health_bar (cast `/Game/UI/WidgetBP/WBP_HealthBar` (`WidgetComponent.GetUserWidgetObject` (`self.HealthBar_0`))))
  (`/Game/UI/WidgetBP/WBP_HealthBar.SetPercentage` _aswbp_health_bar (/ Health MaxHealth)))

(event `self.BP_Die`
  (bind _returnvalue (`self.PlayAnimMontage` "/Game/BluePrint/Character/Animation/AM_Shinbi_Die.AM_Shinbi_Die"))
  (`KismetSystemLibrary.Delay` _returnvalue)
  (`self.K2_DestroyActor`))

(fn `UserConstructionScript`
  (`parent.UserConstructionScript`))