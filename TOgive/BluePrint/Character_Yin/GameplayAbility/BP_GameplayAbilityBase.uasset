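; Base Gameplay Ability Blueprint with shared helpers for player info, UI cooldown and cost checks; its activate and end events are empty.
; GetPlayerInfo casts the owning actor to BP_CharacterBase and its controller to BP_PlayerControllerBase.
; DOUICoollDown starts the cooldown on PrimaryUI slots whose ability class matches this one.
; IsCosrStillAvaluable checks that the Health, Mana or Strength attribute selected by CostType exceeds the negated Cost.
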(fn `DOUICoollDown`
  (bind (_charabase _controllerbase) (`self.GetPlayerInfo`))
  (`/Engine/EditorBlueprintResources/StandardMacros.IsValid` _controllerbase
    (:`Is Valid`
      (for _array_element (`/Game/UI/WBP_PrimaryUI.Slots` (`/Game/BluePrint/BP_PlayerControllerBase.Primary UI` _controllerbase))
        (bind _returnvalue (`self.GetAbilityInfo`))
        (bind (_abilityinfo_cooldownduration _abilityinfo_cost _abilityinfo_costtype _abilityinfo_uimat _abilityinfo_abilityclass) (break `GameplayAbilityInfo` (`/Game/UI/WBP_Ability_Slot.AbilityInfo` _array_element)))
        (if (== _abilityinfo_abilityclass (`.AbilityClass` (break `GameplayAbilityInfo` _returnvalue)))
          (`/Game/UI/WBP_Ability_Slot.StartCoolDown` _array_element))))))

(fn `GetPlayerInfo`
  (returns (Charabase :type "/Game/BluePrint/Character_Yin/BP_CharacterBase Object Reference") (ControllerBase :type "/Game/BluePrint/BP_PlayerControllerBase Object Reference"))
  (bind _asbp_character_base (cast `/Game/BluePrint/Character_Yin/BP_CharacterBase` (`self.GetOwningActorFromActorInfo`)))
  (bind _asbp_player_controller_base (cast `/Game/BluePrint/BP_PlayerControllerBase` (`Pawn.GetController` _asbp_character_base))
    (:`then`
      _)
    (:`CastFailed`
      _))
  (return _asbp_character_base _asbp_player_controller_base))

(fn `IsCosrStillAvaluable`
  (returns (Can :type Boolean))
  (locals (Cost :type "Float (double-precision)"))
  (bind _returnvalue (`self.GetAbilityInfo`))
  (set `local.Cost` (* (`.Cost` (break `GameplayAbilityInfo` _returnvalue)) -1.0))
  (switch `EAbilityCostType` (`.CostType` (break `GameplayAbilityInfo` _returnvalue))
    (:`Health`
      (bind _charabase (`self.GetPlayerInfo`))
      (bind (_health_basevalue _health_currentvalue) (break `GameplayAttributeData` (`MyAttributeSetBase.Health` (`MyCharacterBase.AttributeSetBaseComp` _charabase))))
      (return (> _health_currentvalue (`local.Cost`))))
    (:`Mana`
      (bind _charabase_2 (`self.GetPlayerInfo`))
      (bind (_mana_basevalue _mana_currentvalue) (break `GameplayAttributeData` (`MyAttributeSetBase.Mana` (`MyCharacterBase.AttributeSetBaseComp` _charabase_2))))
      (return (> _mana_currentvalue (`local.Cost`))))
    (:`Strength`
      (bind _charabase_3 (`self.GetPlayerInfo`))
      (bind (_strength_basevalue _strength_currentvalue) (break `GameplayAttributeData` (`MyAttributeSetBase.Strength` (`MyCharacterBase.AttributeSetBaseComp` _charabase_3))))
      (return (> _strength_currentvalue (`local.Cost`))))))