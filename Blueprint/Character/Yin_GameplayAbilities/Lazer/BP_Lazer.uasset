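; BP_Lazer is the laser skill actor that periodically signals damage for hostile characters inside its beam.
; Lazerend overlap events add hostile Yin characters, judged against the instigator, to a unique target array and remove them on exit.
; A looping timer started at BeginPlay packs that array into target data and sends a Skill.lazer.dealDamage gameplay event to the instigator, leaving damage handling outside this actor.
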(event `self.ReceiveBeginPlay`
  (`KismetSystemLibrary.K2_SetTimerDelegate` (delegate `SendDealDamageEvent`) 0.3 true))

(event `SendDealDamageEvent`
  (if (`KismetMathLibrary.Conv_IntToBool` (`KismetArrayLibrary.Array_Length` (`self.OverlapingActor_Yin`)))
    _
    (else
      _))
  (`AbilitySystemBlueprintLibrary.SendGameplayEventToActor` (`self.GetInstigator`) (struct :`TagName` "skill.lazer.dealDamage") (make `GameplayEventData` (struct :`TagName` "skill.lazer.dealDamage") null null null null (struct) (struct) (struct) 0.0 (`AbilitySystemBlueprintLibrary.AbilityTargetDataFromActorArray` (`self.OverlapingActor_Yin`)))))

(event `self.Lazerend.OnComponentBeginOverlap`
  (params (OverlappedComponent :type "PrimitiveComponent Object Reference") (OtherActor :type "Actor Object Reference") (OtherComp :type "PrimitiveComponent Object Reference") (OtherBodyIndex :type Integer) (bFromSweep :type Boolean) (SweepResult :type "HitResult Structure (by ref)"))
  (bind _asbp_yin_characrer_base (cast `/Game/BluePrint/Character/BP_Yin_CharacrerBase` OtherActor))
  (bind _asbp_yin_characrer_base_2 (cast `/Game/BluePrint/Character/BP_Yin_CharacrerBase` (`self.GetInstigator`)))
  (bind _returnvalue (`wzryCharacter.IsOtherHostile` _asbp_yin_characrer_base_2 _asbp_yin_characrer_base))
  (if _returnvalue
    (`KismetArrayLibrary.Array_AddUnique` (`self.OverlapingActor_Yin`) _asbp_yin_characrer_base)))

(event `self.Lazerend.OnComponentEndOverlap`
  (params (OverlappedComponent :type "PrimitiveComponent Object Reference") (OtherActor :type "Actor Object Reference") (OtherComp :type "PrimitiveComponent Object Reference") (OtherBodyIndex :type Integer))
  (bind _asbp_yin_characrer_base (cast `/Game/BluePrint/Character/BP_Yin_CharacrerBase` OtherActor))
  (`KismetArrayLibrary.Array_RemoveItem` (`self.OverlapingActor_Yin`) _asbp_yin_characrer_base))

(fn `UserConstructionScript`)