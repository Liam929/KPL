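; Shinbi's Q dash gameplay ability, which launches the character forward, damaging and knocking back characters it hits.
; Activation commits, triggers the cooldown UI, zeroes ground friction, sets pawn collision to overlap, applies a forward velocity impulse and plays the dash montage.
; Skill.dash.dealDamage events apply the damage effect, then push Shinbi-base targets away with a stun.
; Montage completion, blend-out or interruption restores friction and blocking collision, then ends the ability.
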(event `self.K2_ActivateAbility`
  (`self.K2_CommitAbility`)
  (`self.DoUICD`)
  (bind _ascharacter (cast `Character` (`self.GetOwningActorFromActorInfo`))
    (:`then`
      (bind _charactermovement (`Character.CharacterMovement` _ascharacter))
      (set `self.OriginalGroundFriction` (`CharacterMovementComponent.GroundFriction` _charactermovement))
      (set `CharacterMovementComponent.GroundFriction` 0.0 _charactermovement)
      (`CharacterMovementComponent.AddImpulse` _charactermovement (* (`Actor.GetActorForwardVector` _ascharacter) 900.0) true) ; Don't have vector
      (bind _characterbase (`self.GetCharacterAndController`))
      (`/Game/BluePrint/Character/BP_Shinbi_CharacterBase.SetCollisionToPawn` _characterbase "ECR_Overlap")
      (`AbilityTask_PlayMontageAndWait.CreatePlayMontageAndWaitProxy` "None" "/Game/BluePrint/Character/Animation/AM_Shinbi_Q_Dash.AM_Shinbi_Q_Dash"
        (:`then`
          (bind (_asynctaskproxy _payload) (`AbilityTask_WaitGameplayEvent.WaitGameplayEvent` (struct :`TagName` "skill.dash.dealDamage") null)
            (:`EventReceived`
              (bind (_eventtag _instigator _target) (break `GameplayEventData` _payload))
              (`self.BP_ApplyGameplayEffectToTarget` (`AbilitySystemBlueprintLibrary.AbilityTargetDataFromActor` _target) "/Game/BluePrint/Character/Shinbi_GameplayAbilities/Shinbi_Q_Dash/GE_Shinbi_Dash_Damage.GE_Shinbi_Dash_Damage_C")
              (bind _asbp_shinbi_character_base (cast `/Game/BluePrint/Character/BP_Shinbi_CharacterBase` _target))
              (`/Game/BluePrint/Character/BP_Shinbi_CharacterBase.PushCharacter` _asbp_shinbi_character_base (`KismetMathLibrary.Normal` (- (`Actor.K2_GetActorLocation` _asbp_shinbi_character_base) (`Actor.K2_GetActorLocation` (`self.GetOwningActorFromActorInfo`)))) 1000.0 1.0))))
        (:`OnCompleted`
          (set `CharacterMovementComponent.GroundFriction` (`self.OriginalGroundFriction`) _charactermovement :!label _label)
          (bind _characterbase_2 (`self.GetCharacterAndController`))
          (`/Game/BluePrint/Character/BP_Shinbi_CharacterBase.SetCollisionToPawn` _characterbase_2 "ECR_Block")
          (`self.K2_EndAbility`))
        (:`OnBlendOut`
          (goto _label))
        (:`OnInterrupted`
          (goto _label))
        (:`OnCancelled`
          (goto _label))))
    (:`CastFailed`
      (`self.K2_EndAbility`))))