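; Gameplay ability for Yin's laser attack, which commits, triggers the UI cooldown and plays a casting montage.
; It spawns BP_Lazer on the mesh's Lazer socket and listens for gameplay events carrying target data.
; While cost remains available, each event applies laser damage and a zero-impulse stun via PushCharacter; otherwise the ability ends.
; Montage exit also ends it, and cleanup removes owner effects and destroys the laser.
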(event `self.K2_ActivateAbility`
  (`self.K2_CommitAbility`)
  (`self.DoUICD`)
  (`AbilityTask_PlayMontageAndWait.CreatePlayMontageAndWaitProxy` "None" "/Game/TOGIVE/BluePrint/Character_Yin/Animation/AM_LazerCasting.AM_LazerCasting"
    (:`then`
      (`KismetSystemLibrary.Delay` 0.0)
      (bind _characterbase (`self.GetCharacterAndController`))
      (bind (_asynctaskproxy _spawnedactor) (`AbilityTask_SpawnActor.SpawnActor` (struct) "/Game/BluePrint/Character/Yin_GameplayAbilities/Lazer/BP_Lazer.BP_Lazer_C" _characterbase)
        (:`then`
          (bind _output_get (set `self.LazerActor` _spawnedactor))
          (`Actor.K2_AttachToComponent` _output_get (`Character.Mesh` _characterbase) "Lazer" "SnapToTarget" "SnapToTarget" "KeepRelative" true)
          (bind _asbp_yin_characrer_base (cast `/Game/BluePrint/Character/BP_Yin_CharacrerBase` _characterbase))
          (`/Game/BluePrint/Character/BP_Yin_CharacrerBase.MakeCameraControllRotation` _asbp_yin_characrer_base false)
          (bind (_asynctaskproxy_2 _payload) (`AbilityTask_WaitGameplayEvent.WaitGameplayEvent` (struct) null)
            (:`EventReceived`
              (bind _can (`self.IsCostStillAvaliable`))
              (if _can
                (bind (_eventtag _instigator _target _optionalobject _optionalobject2 _contexthandle _instigatortags _targettags _eventmagnitude _targetdata) (break `GameplayEventData` _payload))
                (`self.BP_ApplyGameplayEffectToTarget` _targetdata "/Game/BluePrint/Character/Yin_GameplayAbilities/Lazer/GE_LazerDamage.GE_LazerDamage_C")
                (for _array_element (`AbilitySystemBlueprintLibrary.GetActorsFromTargetData` _targetdata)
                  (bind _asbp_yin_characrer_base_2 (cast `/Game/BluePrint/Character/BP_Yin_CharacrerBase` _array_element))
                  (`/Game/BluePrint/Character/BP_Shinbi_CharacterBase.PushCharacter` _asbp_yin_characrer_base_2 (0.0 0.0 0.0) 0.0 0.7))
                (else
                  (`self.K2_EndAbility`))))))))
    (:`OnCompleted`
      (`self.K2_EndAbility` :!label _label))
    (:`OnBlendOut`
      (goto _label))
    (:`OnInterrupted`
      (goto _label))
    (:`OnCancelled`
      (goto _label))))

(event `self.K2_OnEndAbility`
  (params (bWasCancelled :type Boolean))
  (`self.BP_RemoveGameplayEffectFromOwnerWithAssetTags` (struct))
  (`Actor.K2_DestroyActor` (`self.LazerActor`))
  (bind _characterbase (`self.GetCharacterAndController`))
  (bind _asbp_yin_characrer_base (cast `/Game/BluePrint/Character/BP_Yin_CharacrerBase` _characterbase))
  (`/Game/BluePrint/Character/BP_Yin_CharacrerBase.MakeCameraControllRotation` _asbp_yin_characrer_base false))